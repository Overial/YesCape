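; BP_PlayerBlue_Character is the blue player character, which carries a flashlight and loses the game when an enemy touches it.
; On BeginPlay it spawns a BP_Flashlight and snaps it to the mesh's FlashlightSocket.
; A capsule hit from an actor tagged Enemy slows global time, switches the mesh to physics ragdoll with movement disabled, and calls OnGameOver(false) on the YesCape player controller.
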(event OnComponentHit(CapsuleComponent)
  (params (HitComponent :type Primitive%20Component%20Object%20Reference) (OtherActor :type Actor%20Object%20Reference) (OtherComp :type Primitive%20Component%20Object%20Reference) (NormalImpulse :type Vector :default "0, 0, 0") (Hit :type Hit%20Result%20Structure%20%28by%20ref%29))
  (Utilities|IsValid OtherActor
    (:Is%20Valid
      (if (Actor|ActorHasTag OtherActor "Enemy")
        (Utilities|Time|SetGlobalTimeDilation 0.5)
        (CallFunction|FnEnableRagdoll)
        (bind _asmaster_bp_yes_cape_player_player_controller (Utilities|Casting|CastToMaster_BP_YesCapePlayer_PlayerController (Game|GetPlayerController 0)))
        (Default|OnGameOver _asmaster_bp_yes_cape_player_player_controller false)))))

(event EventBeginPlay
  (|CallParentFunction)
  (Utilities|FlowControl|Sequence
    (:then_0
      (bind _returnvalue (Game|SpawnActorfromClass "/Game/GameFiles/Blueprints/Device/Flashlight/BP_Flashlight.BP_Flashlight_C" (Math|Transform|MakeTransform (Transformation|GetActorLocation)) "Undefined" 0 0))
      (Transformation|AttachComponentToComponent _returnvalue (Variables|Character|GetMesh) "FlashlightSocket" "SnapToTarget" "SnapToTarget" "SnapToTarget" true))))

(fn ConstructionScript
  (|CallParentFunction))

(fn FnEnableRagdoll
  (bind _mesh (Variables|Character|GetMesh))
  (Collision|SetCollisionEnabled (Variables|Default|GetCapsuleComponent) "NoCollision")
  (Physics|SetSimulatePhysics _mesh true)
  (Class|SkeletalMeshComponent|SetAllBodiesSimulatePhysics _mesh true)
  (Collision|SetCollisionEnabled _mesh "QueryAndPhysics")
  (Collision|SetCollisionResponsetoAllChannels _mesh "ECR_Block")
  (Pawn|Components|CharacterMovement|DisableMovement (Variables|Character|GetCharacterMovement)))