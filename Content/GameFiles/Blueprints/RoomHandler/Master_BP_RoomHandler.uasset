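; Room handler actor that tracks Player and Enemy occupancy by tag and runs a door countdown while the player is inside.
; On BeginPlay it collects overlapping doors and binds their interaction events, closing any open doors whenever one fires.
; A looping one-second timer updates the player display, triggers a random closed, enabled door at zero, then restarts if still occupied.
; Any end overlap clears and resets the timer.
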(event Custom|OnDoorInteracted
  (for _array_element (Variables|Tech|GetDoors)
    (switch Utilities|FlowControl|Switch|SwitchonEDoorState (Variables|/Game/GameFiles/Blueprints/InteractiveEntity/Door/Master_BP_Door.Master_BP_Door_C|GetDoorState _array_element)
      (:NewEnumerator1
        (Default|OnCloseDoor _array_element)))))

(event Custom|OnRoomHandlerBeginOverlap
  (params (OverlappedActor :type Actor%20Object%20Reference) (OtherActor :type Actor%20Object%20Reference))
  (CallFunction|FnSetOccupation OtherActor)
  (if (Variables|Gameplay|GetIsOccupiedByPlayer?)
    (CallFunction|OnSetDoorTimer)))

(event Custom|OnRoomHandlerEndOverlap
  (params (OverlappedActor :type Actor%20Object%20Reference) (OtherActor :type Actor%20Object%20Reference))
  (CallFunction|FnUnsetOccupation OtherActor)
  (Utilities|Time|ClearandInvalidateTimerbyHandle (Variables|Tech|GetDoorTimerHandle))
  (Variables|Tech|SetCurrentSecondsLeft (Variables|Gameplay|GetSecondsLeft)))

(event Custom|OnDoorTimerTick
  (bind _closeddoors (Variables|Tech|GetClosedDoors))
  (Variables|Tech|SetCurrentSecondsLeft (- (Variables|Tech|GetCurrentSecondsLeft) 1.0))
  (bind _playerdisplay (Variables|Tech|GetPlayerDisplay)
    (:then
      (Default|OnUpdateTimerInfo _playerdisplay (Variables|Tech|GetCurrentSecondsLeft))
      (if (<= (Variables|Tech|GetCurrentSecondsLeft) 0.0)
        (Utilities|FlowControl|Sequence
          (:then_0
            (Utilities|Array|Clear (Variables|Tech|GetClosedDoors))
            (for _array_element (Variables|Tech|GetDoors)
              (switch Utilities|FlowControl|Switch|SwitchonEDoorState (Variables|/Game/GameFiles/Blueprints/InteractiveEntity/Door/Master_BP_Door.Master_BP_Door_C|GetDoorState _array_element)
                (:NewEnumerator0
                  (if (not (Variables|/Game/GameFiles/Blueprints/InteractiveEntity/Door/Master_BP_Door.Master_BP_Door_C|GetIsDisabled? _array_element))
                    (Utilities|Array|Add (Variables|Tech|GetClosedDoors) _array_element))))))
          (:then_1
            (Class|BPIInteraction|OnInteract(Message) (Utilities|Array|Get(acopy) _closeddoors (Math|Random|RandomInteger (Utilities|Array|Length _closeddoors)))))
          (:then_2
            (Utilities|Time|ClearandInvalidateTimerbyHandle (Variables|Tech|GetDoorTimerHandle))
            (Variables|Tech|SetCurrentSecondsLeft (Variables|Gameplay|GetSecondsLeft)))
          (:then_3
            (if (Variables|Gameplay|GetIsOccupiedByPlayer?)
              (CallFunction|OnSetDoorTimer))))))
    (:else)))

(event Custom|OnSetDoorTimer
  (bind _secondsleft (Variables|Gameplay|GetSecondsLeft))
  (bind _returnvalue (Utilities|Time|SetTimerbyEvent (delegate Custom|OnDoorTimerTick) 1.0 true))
  (Variables|Tech|SetDoorTimerHandle _returnvalue)
  (bind _playerdisplay (Variables|Tech|GetPlayerDisplay)
    (:then
      (Default|OnUpdateTimerInfo _playerdisplay _secondsleft)
      (Variables|Tech|SetCurrentSecondsLeft _secondsleft))
    (:else)))

(event EventBeginPlay
  (Utilities|FlowControl|Sequence
    (:then_0
      (for _array_element (Collision|GetOverlappingActors 0 :!class /Script/Engine.Actor)
        (bind _asmaster_bp_door (Utilities|Casting|CastToMaster_BP_Door _array_element))
        (EventDispatchers|BindEventtoFonDoorInteracted _asmaster_bp_door (delegate Custom|OnDoorInteracted))
        (Utilities|Array|Add (Variables|Tech|GetDoors) _asmaster_bp_door)))
    (:then_1
      (CallFunction|OnSetPlayerDetection))
    (:then_2
      (Collision|BindEventtoOnActorBeginOverlap (delegate Custom|OnRoomHandlerBeginOverlap)))
    (:then_3
      (Collision|BindEventtoOnActorEndOverlap (delegate Custom|OnRoomHandlerEndOverlap)))))

(fn ConstructionScript)

(fn FnonBeginOverlap
  (params (OtherActor :type Actor%20Object%20Reference))
  (Utilities|IsValid OtherActor
    (:Is%20Valid
      (if (Actor|ActorHasTag OtherActor "Player")
        _))))

(fn FnonEndOverlap
  (params (OtherActor :type Actor%20Object%20Reference))
  (Utilities|IsValid OtherActor
    (:Is%20Valid
      (if (Actor|ActorHasTag OtherActor "Player")
        _))))

(fn FnSetOccupation
  (params (OtherActor :type Actor%20Object%20Reference))
  (Utilities|FlowControl|Sequence
    (:then_0
      (if (Actor|ActorHasTag OtherActor "Player")
        (Variables|Gameplay|SetIsOccupiedByPlayer? true)))
    (:then_1
      (if (Actor|ActorHasTag OtherActor "Enemy")
        (Variables|Gameplay|SetIsOccupiedByEnemy? true)))))

(fn FnUnsetOccupation
  (params (OtherActor :type Actor%20Object%20Reference))
  (Utilities|FlowControl|Sequence
    (:then_0
      (if (Actor|ActorHasTag OtherActor "Player")
        (Variables|Gameplay|SetIsOccupiedByPlayer? false)))
    (:then_1
      (if (Actor|ActorHasTag OtherActor "Enemy")
        (Variables|Gameplay|SetIsOccupiedByEnemy? false)))))