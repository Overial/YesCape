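; Base Blueprint for interactive entities that detects when an actor tagged "User" enters or leaves its box collision.
; On overlap begin and end it sets the user's interacting state through message calls and passes the user's tags to OnHandleActorTags.
; Leaving the box also hides and clears the user's interaction message; this graph never shows that message or defines the tag handling.
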(event OnComponentBeginOverlap(EntityBoxCollision)
  (params (OverlappedComponent :type Primitive%20Component%20Object%20Reference) (OtherActor :type Actor%20Object%20Reference) (OtherComp :type Primitive%20Component%20Object%20Reference) (OtherBodyIndex :type Integer) (bFromSweep :type Boolean) (SweepResult :type Hit%20Result%20Structure%20%28by%20ref%29))
  (if (Actor|ActorHasTag OtherActor "User")
    (Class|BPIInteraction|OnSetIsInteracting(Message) OtherActor true)
    (CallFunction|OnHandleActorTags (Variables|/Script/Engine.Actor|GetTags OtherActor))))

(event OnComponentEndOverlap(EntityBoxCollision)
  (params (OverlappedComponent :type Primitive%20Component%20Object%20Reference) (OtherActor :type Actor%20Object%20Reference) (OtherComp :type Primitive%20Component%20Object%20Reference) (OtherBodyIndex :type Integer))
  (if (Actor|ActorHasTag OtherActor "User")
    (Class|BPIInteraction|OnSetIsInteracting(Message) OtherActor false)
    (CallFunction|OnHandleActorTags (Variables|/Script/Engine.Actor|GetTags OtherActor))
    (Class|BPIInteraction|OnSetInteractionMessage(Message) OtherActor "Hidden" "")))

(fn ConstructionScript)