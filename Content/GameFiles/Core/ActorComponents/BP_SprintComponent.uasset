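; BP_SprintComponent is an actor component that switches its owning Character between walking and sprinting speeds.
; On BeginPlay it casts the owner to Character and caches its movement component, stopping if the cast fails.
; The OnStartSprint and OnStopSprint events then set MaxWalkSpeed to the sprinting or walking value, guarded by a validity check on the cached movement component.
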(event Custom|OnStartSprint
  (bind _currentcharactermovement (Variables|Default|GetCurrentCharacterMovement)
    (:then
      (Variables|/Script/Engine.CharacterMovementComponent|SetMaxWalkSpeed _currentcharactermovement (Variables|Default|GetSprintingSpeed)))
    (:else)))

(event Custom|OnStopSprint
  (bind _currentcharactermovement (Variables|Default|GetCurrentCharacterMovement)
    (:then
      (Variables|/Script/Engine.CharacterMovementComponent|SetMaxWalkSpeed _currentcharactermovement (Variables|Default|GetWalkingSpeed)))
    (:else)))

(event EventBeginPlay
  (bind _ascharacter (Utilities|Casting|CastToCharacter (Components|GetOwner)))
  (Variables|Default|SetCurrentCharacterMovement (Variables|/Script/Engine.Character|GetCharacterMovement _ascharacter)))